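; Child block Blueprint, apparently a destructible block variant that shrinks slightly on its first hit before deferring to its parent's overlap behavior.
; BeginPlay runs the parent logic and caches the starting scale.
; The first actor overlap passes through a DoOnce, reduces scale by a small fraction of the original and sets the Smalled flag.
; Later overlaps are forwarded to the parent's overlap handler.
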(event `self.ReceiveBeginPlay`
  (`parent.ReceiveBeginPlay`)
  (set `self.InitScale` (`self.GetActorScale3D`)))

(event `self.ReceiveActorBeginOverlap`
  (params (OtherActor :type "Actor Object Reference"))
  (if (`self.smalled?`)
    (`parent.ReceiveActorBeginOverlap` OtherActor)
    (else
      (`/Engine/EditorBlueprintResources/StandardMacros.DoOnce` false
        (:`Completed`
          (`self.SetActorScale3D` (- (`self.GetActorScale3D`) (* (`self.InitScale`) 0.05)))
          (set `self.smalled?` true))))))

(fn `UserConstructionScript`
  (`parent.UserConstructionScript`))